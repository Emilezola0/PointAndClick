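; Interactive painting for an ordered-sequence quest puzzle that opens a door.
; Interacting in order arms the next linked painting; the last opens the door, sets the Quest.Painting tag and plays finish dialogue, which replays on later interactions.
; An out-of-order interaction plays fail dialogue from DT_Dialogue, then clears the progress flag on every painting in AllPainting.
; Player interaction is locked during dialogue, and the construction script applies each painting's material.
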(event EventBeginPlay
  (|CallParentFunction))

(event EventCanInteract
  (params (CharaLooking :type Character%20Object%20Reference))
  (|CallParentFunction CharaLooking))

(event EventInteract
  ;[1 1 1] Interactions
  (if (Variables|/Game/FirstPersonCharacter.FirstPersonCharacter_C|GetcanInteract? (Variables|Default|GetAs%20First%20Person%20Character))
    (Variables|/Game/FirstPersonCharacter.FirstPersonCharacter_C|SetcanInteract? (Variables|Default|GetAs%20First%20Person%20Character) false)
    (if (CallFunction|HaveTag "(TagName=\"Quest.Painting\")")
      (bind _returnvalue (Utilities|GetDataTableRow "/Game/DialogueSystem/DT_Dialogue.DT_Dialogue" "QuestPaintingFinish" :!label _label)
        (:then
          (bind _delay_before_remove_widget (CallFunction|Dialogue (.Name (Utilities|Struct|BreakSDialogue _returnvalue)) (.Text (Utilities|Struct|BreakSDialogue _returnvalue)) (.TextSpeed (Utilities|Struct|BreakSDialogue _returnvalue)) (.3DSound? (Utilities|Struct|BreakSDialogue _returnvalue)) (.Sound (Utilities|Struct|BreakSDialogue _returnvalue)) (.VolumeMultiplier (Utilities|Struct|BreakSDialogue _returnvalue)) (.PitchMultiplier (Utilities|Struct|BreakSDialogue _returnvalue)) (Transformation|GetActorLocation) (.AutomaticalyRemoveAtEnd? (Utilities|Struct|BreakSDialogue _returnvalue)) (.DelayIfNoSound (Utilities|Struct|BreakSDialogue _returnvalue))))
          (Utilities|FlowControl|Delay _delay_before_remove_widget)
          (Variables|/Game/FirstPersonCharacter.FirstPersonCharacter_C|SetcanInteract? (Variables|Default|GetAs%20First%20Person%20Character) true)))
      (elif (Variables|PaintingParameter|GetHaveInteractWithTheOneBefore?)
        (if (Variables|PaintingParameter|GetIsTheLastPainting?)
          (Default|OpenDoor (Variables|PaintingParameter|GetDoorToOpen))
          (CallFunction|SetTag "(TagName=\"Quest.Painting\")")
          (goto _label)
          (else
            (Variables|BP_BaseInteractiveActor_ChildPainting_C|SetHaveInteractWithTheOneBefore? (Variables|PaintingParameter|GetPaintingToInteractAfter) true)
            (Variables|/Game/FirstPersonCharacter.FirstPersonCharacter_C|SetcanInteract? (Variables|Default|GetAs%20First%20Person%20Character) true)))
        (else
          (bind _returnvalue_2 (Utilities|GetDataTableRow "/Game/DialogueSystem/DT_Dialogue.DT_Dialogue" (Variables|PaintingParameter|GetFailDialogueName))
            (:then
              (bind _delay_before_remove_widget_2 (CallFunction|Dialogue (.Name (Utilities|Struct|BreakSDialogue _returnvalue_2)) (.Text (Utilities|Struct|BreakSDialogue _returnvalue_2)) (.TextSpeed (Utilities|Struct|BreakSDialogue _returnvalue_2)) (.3DSound? (Utilities|Struct|BreakSDialogue _returnvalue_2)) (.Sound (Utilities|Struct|BreakSDialogue _returnvalue_2)) (.VolumeMultiplier (Utilities|Struct|BreakSDialogue _returnvalue_2)) (.PitchMultiplier (Utilities|Struct|BreakSDialogue _returnvalue_2)) (Transformation|GetActorLocation) (.AutomaticalyRemoveAtEnd? (Utilities|Struct|BreakSDialogue _returnvalue_2)) (.DelayIfNoSound (Utilities|Struct|BreakSDialogue _returnvalue_2))))
              (Utilities|FlowControl|Delay _delay_before_remove_widget_2)
              (for _array_element (Variables|PaintingParameter|GetAllPainting)
                (Variables|BP_BaseInteractiveActor_ChildPainting_C|SetHaveInteractWithTheOneBefore? _array_element false))
              (Variables|/Game/FirstPersonCharacter.FirstPersonCharacter_C|SetcanInteract? (Variables|Default|GetAs%20First%20Person%20Character) true))))))))

(fn ConstructionScript
  (Rendering|Material|SetMaterial (Variables|Default|Getdesign) 0 (Variables|Default|GetMaterial))
  (|CallParentFunction))