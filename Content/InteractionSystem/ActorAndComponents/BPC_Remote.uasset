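; Player controller component that acts as a teleport remote for the first-person character.
; On BeginPlay it caches the character and adds the interactions Enhanced Input mapping context.
; The first-use input calls TP to swap positions with the character's ChildRef actor when valid.
; Otherwise, a FlipFlop alternately shifts the character up and down by a fixed vertical offset.
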(event Input|EnhancedActionEvents|EnhancedInputActionIA_FirstUse
  (params (ActionValue :type Boolean) (ElapsedSeconds :type Float%20%28double-precision%29) (TriggeredSeconds :type Float%20%28double-precision%29) (InputAction :type Input%20Action%20Object%20Reference :default "/Game/InputSystem/Actions/IA_FirstUse.IA_FirstUse"))
  (:Triggered
    (Utilities|IsValid (Variables|/Game/FirstPersonCharacter.FirstPersonCharacter_C|GetChildRef (Variables|Default|GetAs%20First%20Person%20Character))
      (:Is%20Valid
        (|TP))
      (:Is%20Not%20Valid
        (Utilities|FlowControl|FlipFlop
          (:A
            (Transformation|SetActorLocation (Variables|Default|GetAs%20First%20Person%20Character) (+ (Transformation|GetActorLocation (Variables|Default|GetAs%20First%20Person%20Character)) "0.000000,0.000000,1500.000000") false false))
          (:B
            (Transformation|SetActorLocation (Variables|Default|GetAs%20First%20Person%20Character) (+ (Transformation|GetActorLocation (Variables|Default|GetAs%20First%20Person%20Character)) "0.000000,0.000000,-1500.000000") false false)))))))

(event EventBeginPlay
  (bind _asfirst_person_character (Utilities|Casting|CastToFirstPersonCharacter (Game|GetPlayerCharacter 0)))
  (Variables|Default|SetAs%20First%20Person%20Character _asfirst_person_character)
  (bind _asplayer_controller (Utilities|Casting|CastToPlayerController (Components|GetOwner)))
  (Utilities|IsValid (PlayerController|LocalPlayerSubsystems|GetEnhancedInputLocalPlayerSubsystem _asplayer_controller)
    (:Is%20Valid
      (Input|AddMappingContext (PlayerController|LocalPlayerSubsystems|GetEnhancedInputLocalPlayerSubsystem _asplayer_controller) "/Game/InputSystem/IMC_Interactions.IMC_Interactions" 0 "(bIgnoreAllPressedKeysUntilRelease=True,bForceImmediately=False)"))))