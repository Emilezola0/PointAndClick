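; Interactive actor Blueprint, named as the Remote variant, that works as a single-use interactable removed from the world when used.
; On Interact, it checks the first-person character's CanInteract flag and sets it to false.
; It then hides itself, runs the parent Interact logic and destroys the actor.
; BeginPlay, CanInteract and construction only forward to the parent class.
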(event EventBeginPlay
  (|CallParentFunction))

(event EventCanInteract
  (params (CharaLooking :type Character%20Object%20Reference))
  (|CallParentFunction CharaLooking))

(event EventInteract
  (if (Variables|/Game/FirstPersonCharacter.FirstPersonCharacter_C|GetcanInteract? (Variables|Default|GetAs%20First%20Person%20Character))
    (Variables|/Game/FirstPersonCharacter.FirstPersonCharacter_C|SetcanInteract? (Variables|Default|GetAs%20First%20Person%20Character) false)
    (Rendering|SetActorHiddenInGame true)
    (|CallParentFunction)
    (Actor|DestroyActor)))

(fn ConstructionScript
  (|CallParentFunction))