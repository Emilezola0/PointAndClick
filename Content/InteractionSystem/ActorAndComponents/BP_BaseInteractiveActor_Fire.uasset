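; Interactive fire actor that plays a hint dialogue until the player has the Quest.SecondWindows tag, apparently pointing toward the secret-code puzzle.
; Interact locks the first-person character's CanInteract, then feeds the IndiceFireScene1 row from DT_Dialogue into Dialogue at the actor's location.
; Interaction unlocks after the delay that Dialogue returns.
; With the tag present or the row missing, this graph never restores CanInteract.
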(event EventBeginPlay
  (|CallParentFunction))

(event EventCanInteract
  (params (CharaLooking :type Character%20Object%20Reference))
  (|CallParentFunction CharaLooking))

(event EventInteract
  (if (Variables|/Game/FirstPersonCharacter.FirstPersonCharacter_C|GetcanInteract? (Variables|Default|GetAs%20First%20Person%20Character))
    (Variables|/Game/FirstPersonCharacter.FirstPersonCharacter_C|SetcanInteract? (Variables|Default|GetAs%20First%20Person%20Character) false)
    (if (not (CallFunction|HaveTag "(TagName=\"Quest.SecondWindows\")"))
      ;[1 1 1] Indice for the bloody text & paint for a secret code you have second windows when you finish the code
      (bind _returnvalue (Utilities|GetDataTableRow "/Game/DialogueSystem/DT_Dialogue.DT_Dialogue" (Variables|Default|GetIndiceFireScene1))
        (:then
          (bind _delay_before_remove_widget (CallFunction|Dialogue (.Name (Utilities|Struct|BreakSDialogue _returnvalue)) (.Text (Utilities|Struct|BreakSDialogue _returnvalue)) (.TextSpeed (Utilities|Struct|BreakSDialogue _returnvalue)) (.3DSound? (Utilities|Struct|BreakSDialogue _returnvalue)) (.Sound (Utilities|Struct|BreakSDialogue _returnvalue)) (.VolumeMultiplier (Utilities|Struct|BreakSDialogue _returnvalue)) (.PitchMultiplier (Utilities|Struct|BreakSDialogue _returnvalue)) (Transformation|GetActorLocation) (.AutomaticalyRemoveAtEnd? (Utilities|Struct|BreakSDialogue _returnvalue)) (.DelayIfNoSound (Utilities|Struct|BreakSDialogue _returnvalue))))
          (Utilities|FlowControl|Delay _delay_before_remove_widget)
          (Variables|/Game/FirstPersonCharacter.FirstPersonCharacter_C|SetcanInteract? (Variables|Default|GetAs%20First%20Person%20Character) true))))))

(fn ConstructionScript
  (|CallParentFunction))