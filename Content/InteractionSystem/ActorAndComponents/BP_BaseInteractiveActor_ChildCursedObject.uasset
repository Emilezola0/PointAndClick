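; Child interactive actor for a cursed object that plays a dialogue line when the player interacts with it.
; Interact looks up its row in DT_Dialogue and passes the text, speaker, typing and sound settings to Dialogue at the actor's location.
; It blocks further player interaction and sets the narrator-sound flag, then restores both after the delay Dialogue returns.
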(event EventBeginPlay
  (|CallParentFunction))

(event EventInteract
  ;[1 1 1] Interactions
  (if (Variables|/Game/FirstPersonCharacter.FirstPersonCharacter_C|GetcanInteract? (Variables|Default|GetAs%20First%20Person%20Character))
    (Variables|/Game/FirstPersonCharacter.FirstPersonCharacter_C|SetcanInteract? (Variables|Default|GetAs%20First%20Person%20Character) false)
    (bind _returnvalue (Utilities|GetDataTableRow "/Game/DialogueSystem/DT_Dialogue.DT_Dialogue" (Variables|Default|GetRow%20Name))
      (:then
        (bind (_delay_before_remove_widget _widget_reference _isplayingsound_) (CallFunction|Dialogue (.Name (Utilities|Struct|BreakSDialogue _returnvalue)) (.Text (Utilities|Struct|BreakSDialogue _returnvalue)) (.TextSpeed (Utilities|Struct|BreakSDialogue _returnvalue)) (.3DSound? (Utilities|Struct|BreakSDialogue _returnvalue)) (.Sound (Utilities|Struct|BreakSDialogue _returnvalue)) (.VolumeMultiplier (Utilities|Struct|BreakSDialogue _returnvalue)) (.PitchMultiplier (Utilities|Struct|BreakSDialogue _returnvalue)) (Transformation|GetActorLocation) (.AutomaticalyRemoveAtEnd? (Utilities|Struct|BreakSDialogue _returnvalue)) (.DelayIfNoSound (Utilities|Struct|BreakSDialogue _returnvalue))))
        (Variables|/Game/FirstPersonCharacter.FirstPersonCharacter_C|SethaveNarratorSound? (Variables|Default|GetAs%20First%20Person%20Character) _isplayingsound_)
        (Utilities|FlowControl|Delay _delay_before_remove_widget)
        (Variables|/Game/FirstPersonCharacter.FirstPersonCharacter_C|SetcanInteract? (Variables|Default|GetAs%20First%20Person%20Character) true)
        (Variables|/Game/FirstPersonCharacter.FirstPersonCharacter_C|SethaveNarratorSound? (Variables|Default|GetAs%20First%20Person%20Character) false)))))

(event EventCanInteract
  (params (CharaLooking :type Character%20Object%20Reference))
  (|CallParentFunction CharaLooking))

(fn ConstructionScript
  (|CallParentFunction))