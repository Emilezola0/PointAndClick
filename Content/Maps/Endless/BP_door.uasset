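; BP_door is a sliding door in the Endless map folder that moves its Cube vertically between open and closed heights.
; BeginPlay records the cube's starting Z and adds DoorDistance to get the final height.
; OpenDoor and CloseDoor events each play their own timeline, easing Z with ExpoInOut toward the final or starting height.
; Leftover Character-cast, DoOnce triggers are disconnected, so nothing in this graph calls either event at runtime.
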(event Custom|OpenDoor
  (bind _cube (Variables|Default|GetCube))
  (bind _returnvalue (Transformation|GetWorldLocation _cube))
  (bind _alpha (Timeline|Timeline PlayFromStart)
    (:Update
      (Transformation|SetWorldLocation _cube (Math|Vector|MakeVector (.x _returnvalue) (.y _returnvalue) (Math|Interpolation|Ease "ExpoInOut" _alpha (Variables|Default|GetStart_location) (Variables|Default|GetFinal_location))) false false))))

(event Custom|CloseDoor
  (bind _cube (Variables|Default|GetCube))
  (bind _final_location (Variables|Default|GetFinal_location))
  (bind _returnvalue (Transformation|GetWorldLocation _cube))
  (bind _alpha (Timeline|Timeline_0 PlayFromStart)
    (:Update
      (Transformation|SetWorldLocation _cube (Math|Vector|MakeVector (.x _returnvalue) (.y _returnvalue) (Math|Interpolation|Ease "ExpoInOut" _alpha _final_location (- _final_location (Variables|Default|GetDoorDistance)))) false false))))

(event EventBeginPlay
  (bind _cube (Variables|Default|GetCube))
  (bind _returnvalue (Transformation|GetWorldLocation _cube))
  (Variables|Default|SetStart_location (.z _returnvalue))
  (Variables|Default|SetFinal_location (+ (.z _returnvalue) (Variables|Default|GetDoorDistance))))

(fn ConstructionScript)