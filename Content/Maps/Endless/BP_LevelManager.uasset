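; Level manager for an endless anomaly-spotting corridor that streams rooms and scores the player's choices.
; LoadNextCorridor raises RoomCount when the player's SwitchDimension matches the anomaly flag and resets it otherwise, with audio feedback; a count of six jumps straight to 666.
; It places a uniquely named CorridorRoom streaming instance at the given transform and clears SwitchDimension.
; UnloadPreviousCorridor removes the oldest stored room once RoomCount exceeds two.
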(event EventBeginPlay
  (bind _returnvalue (Actor|GetActorOfClass "/Game/FirstPersonCharacter.FirstPersonCharacter_C"))
  (Variables|Default|SetPlayer _returnvalue))

(fn ConstructionScript)

(fn LoadNextCorridor
  (params (LevelLocation :type Vector) (LevelRotation :type Rotator) (Anomalie :type Boolean))
  (bind _asbp_sea_of_love_game_instance (CallFunction|GetInst))
  (bind _asbp_sea_of_love_game_instance_2 (CallFunction|GetInst))
  (if (== (Variables|/Game/Core/BP_SeaOfLoveGameInstance.BP_SeaOfLoveGameInstance_C|GetRoomCount _asbp_sea_of_love_game_instance) 6)
    (Variables|/Game/Core/BP_SeaOfLoveGameInstance.BP_SeaOfLoveGameInstance_C|SetRoomCount _asbp_sea_of_love_game_instance 666)
    (Audio|PlaySound2D "/Game/Sound/CorrectAnswer_Cue.CorrectAnswer_Cue" 1.0 0.6 0.0 0 0)
    (bind _returnvalue (Class|LevelStreaming|CreateInstance (Class|GameplayStatics|GetStreamingLevel "CorridorRoom") (Utilities|String|Append "Room -" (Guid|ToString(Guid) (Guid|NewGuid)))))
    (Variables|Default|SetSelectIndex 0)
    (elif (and Anomalie (Variables|/Game/FirstPersonCharacter.FirstPersonCharacter_C|GetSwitchDimension (Variables|Default|GetPlayer)))
      (Variables|/Game/Core/BP_SeaOfLoveGameInstance.BP_SeaOfLoveGameInstance_C|SetRoomCount _asbp_sea_of_love_game_instance_2 (+ (Variables|/Game/Core/BP_SeaOfLoveGameInstance.BP_SeaOfLoveGameInstance_C|GetRoomCount _asbp_sea_of_love_game_instance_2) 1) :!label _label)
      (Audio|PlaySound2D "/Game/Sound/CorrectAnswer_Cue.CorrectAnswer_Cue" 1.0 1.0 0.0 0 0)
      (bind _returnvalue_2 (Class|LevelStreaming|CreateInstance (Class|GameplayStatics|GetStreamingLevel "CorridorRoom") (Utilities|String|Append "Room -" (Guid|ToString(Guid) (Guid|NewGuid)))))
      (Variables|Default|SetSelectIndex 1)
      (elif (== Anomalie (Variables|/Game/FirstPersonCharacter.FirstPersonCharacter_C|GetSwitchDimension (Variables|Default|GetPlayer)))
        (goto _label)
        (else
          (Variables|/Game/Core/BP_SeaOfLoveGameInstance.BP_SeaOfLoveGameInstance_C|SetRoomCount _asbp_sea_of_love_game_instance_2 0)
          (Audio|PlaySound2D "/Game/Sound/WrongAnswer_Cue.WrongAnswer_Cue" 1.0 1.0 0.0 0 0)
          (bind _returnvalue_3 (Class|LevelStreaming|CreateInstance (Class|GameplayStatics|GetStreamingLevel "CorridorRoom") (Utilities|String|Append "Room -" (Guid|ToString(Guid) (Guid|NewGuid)))))
          (Variables|Default|SetSelectIndex 2)))))
  (Utilities|Array|Add (Variables|Default|GetCorridorXRef) (Utilities|Select :Index (Variables|Default|GetSelectIndex) :Option%200 _returnvalue :Option%201 _returnvalue_2 :Option%202 _returnvalue_3))
  (Variables|/Script/Engine.LevelStreaming|SetbShouldBeLoaded (Utilities|Select :Index (Variables|Default|GetSelectIndex) :Option%200 _returnvalue :Option%201 _returnvalue_2 :Option%202 _returnvalue_3) true)
  (Variables|/Script/Engine.LevelStreaming|SetbShouldBeVisible (Utilities|Select :Index (Variables|Default|GetSelectIndex) :Option%200 _returnvalue :Option%201 _returnvalue_2 :Option%202 _returnvalue_3) true)
  (Variables|/Script/Engine.LevelStreaming|SetbShouldBlockOnLoad (Utilities|Select :Index (Variables|Default|GetSelectIndex) :Option%200 _returnvalue :Option%201 _returnvalue_2 :Option%202 _returnvalue_3) false)
  (Variables|/Script/Engine.LevelStreaming|SetLevelTransform (Utilities|Select :Index (Variables|Default|GetSelectIndex) :Option%200 _returnvalue :Option%201 _returnvalue_2 :Option%202 _returnvalue_3) (Math|Transform|MakeTransform LevelLocation LevelRotation "1.000000,1.000000,1.000000"))
  (Variables|/Game/FirstPersonCharacter.FirstPersonCharacter_C|SetSwitchDimension (Variables|Default|GetPlayer) false)
  (return (Utilities|Select :Index (Variables|Default|GetSelectIndex) :Option%200 _returnvalue :Option%201 _returnvalue_2 :Option%202 _returnvalue_3)))

(fn UnloadPreviousCorridor
  (if (> (Variables|/Game/Core/BP_SeaOfLoveGameInstance.BP_SeaOfLoveGameInstance_C|GetRoomCount (CallFunction|GetInst)) 2)
    (Class|LevelStreaming|SetIsRequestingUnloadandRemoval (Utilities|Array|Get(acopy) (Variables|Default|GetCorridorXRef)) true)
    (Utilities|Array|RemoveIndex (Variables|Default|GetCorridorXRef))))