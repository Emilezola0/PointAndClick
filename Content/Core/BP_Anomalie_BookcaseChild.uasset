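; BP_Anomalie_BookcaseChild is a child anomaly Blueprint for a bookcase that makes its books visible when the anomaly triggers.
; CheckAnomalie calls HiddenFromYourView only when both CanAct and IsAnomalie are true.
; That graph passes each book component to a SetHidden helper, which sets Hidden In Game to false without propagating to children, so it reveals them despite the names.
; BeginPlay and the construction script defer to the parent.
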(event EventBeginPlay
  (|CallParentFunction))

(event EventCheckAnomalie
  (if (Variables|Default|GetbCanAct)
    (if (Variables|Default|GetIsAnomalie?)
      (|HiddenFromYourView))))

(fn ConstructionScript
  (|CallParentFunction))

(fn SetHidden
  (params (Target :type Scene%20Component%20Object%20Reference))
  (Development|SetHiddeninGame Target false false))