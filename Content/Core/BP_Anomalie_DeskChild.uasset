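; Desk anomaly Blueprint, a child actor that can alter itself when its anomaly check runs.
; CheckAnomalie acts only when CanAct and IsAnomalie are true, then picks one of two changes at random.
; It either moves the whole desk straight up without sweeping, or unhides its WANTED component.
; BeginPlay and the construction script only call the parent.
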(event EventBeginPlay
  (|CallParentFunction))

(event EventCheckAnomalie
  (if (Variables|Default|GetbCanAct)
    (if (Variables|Default|GetIsAnomalie?)
      (if (Math|Random|RandomBool)
        (Transformation|SetActorLocation (+ (Transformation|GetActorLocation) "0.000000,0.000000,200.000000") false false)
        (else
          (Development|SetHiddeninGame (Variables|Default|GetWANTED) false false))))))

(fn ConstructionScript
  (|CallParentFunction))