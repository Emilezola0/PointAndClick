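; BP_Anomalie_ChairChild is a child anomaly Blueprint, apparently for a chair that turns into a physics object when it is anomalous.
; CheckAnomalie acts only when CanAct and IsAnomalie are both true, enabling physics simulation on StaticMesh and setting it to block the PhysicsBody channel.
; BeginPlay and the construction script only call the parent versions.
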(event EventBeginPlay
  (|CallParentFunction))

(event EventCheckAnomalie
  (bind _staticmesh (Variables|Default|GetStaticMesh))
  (if (Variables|Default|GetbCanAct)
    (if (Variables|Default|GetIsAnomalie?)
      (Physics|SetSimulatePhysics _staticmesh true)
      (Collision|SetCollisionResponsetoChannel _staticmesh "ECC_PhysicsBody" "ECR_Block"))))

(fn ConstructionScript
  (|CallParentFunction))