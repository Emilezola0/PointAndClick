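; Light variant of an anomaly Blueprint that signals an anomaly by changing the color of its point light.
; CheckAnomalie acts only when CanAct and IsAnomalie are both true, then uses nested random booleans to pick one of four saturated colors with equal odds.
; BeginPlay and the construction script only call the parent, and no graph here restores the original color.
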(event EventBeginPlay
  (|CallParentFunction))

(event EventCheckAnomalie
  (if (Variables|Default|GetbCanAct)
    (if (Variables|Default|GetIsAnomalie?)
      (if (Math|Random|RandomBool)
        (if (Math|Random|RandomBool)
          (Rendering|Components|Light|SetLightColor (Variables|Default|GetPointLight) "(R=1.000000,G=0.073298,B=0.000000,A=1.000000)" true)
          (else
            (Rendering|Components|Light|SetLightColor (Variables|Default|GetPointLight) "(R=1.000000,G=0.000000,B=0.758681,A=1.000000)" true)))
        (elif (Math|Random|RandomBool)
          (Rendering|Components|Light|SetLightColor (Variables|Default|GetPointLight) "(R=0.154099,G=1.000000,B=0.000000,A=1.000000)" true)
          (else
            (Rendering|Components|Light|SetLightColor (Variables|Default|GetPointLight) "(R=0.000000,G=0.011149,B=1.000000,A=1.000000)" true)))))))

(fn ConstructionScript
  (|CallParentFunction))