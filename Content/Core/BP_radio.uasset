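; BP_radio is a world radio that plays an old-time radio playlist with commercials as attenuated 3D audio at its location.
; Five seconds after BeginPlay it spawns and plays the cue; both Otherdimension branches currently use the same sound and settings.
; Tick polls the player FirstPersonCharacter's HaveNarratorSound flag and ducks the radio to near silence while it is set, restoring full volume otherwise.
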(event EventBeginPlay
  (bind _returnvalue (Transformation|GetActorLocation))
  (bind _asfirst_person_character (Utilities|Casting|CastToFirstPersonCharacter (Game|GetPlayerCharacter 0))
    (:then
      (Variables|Default|SetrefChara _asfirst_person_character))
    (:CastFailed
      _))
  (Utilities|FlowControl|Delay 5.0)
  (if (Variables|Default|GetOtherdimension)
    (bind _returnvalue_2 (Audio|SpawnSoundatLocation "/Game/Core/Old_Time_Vintage_Radio_Playlist_with_Commercials_📻_Cue_2.Old_Time_Vintage_Radio_Playlist_with_Commercials_📻_Cue_2" _returnvalue "0, 0, 0" 1.0 1.0 0.0 "/Game/Core/SA_radio.SA_radio" 0 false))
    (bind _output_get (Variables|Default|SetSound _returnvalue_2))
    (Audio|Components|Audio|Play _output_get 0.0)
    (else
      (bind _returnvalue_3 (Audio|SpawnSoundatLocation "/Game/Core/Old_Time_Vintage_Radio_Playlist_with_Commercials_📻_Cue_2.Old_Time_Vintage_Radio_Playlist_with_Commercials_📻_Cue_2" _returnvalue "0, 0, 0" 1.0 1.0 0.0 "/Game/Core/SA_radio.SA_radio" 0 false))
      (bind _output_get_2 (Variables|Default|SetSound _returnvalue_3))
      (Audio|Components|Audio|Play _output_get_2 0.0))))

(event EventTick
  (params (DeltaSeconds :type Float%20%28single-precision%29))
  (bind _sound (Variables|Default|GetSound))
  (Utilities|IsValid (Variables|Default|GetSound)
    (:Is%20Valid
      (if (Variables|/Game/FirstPersonCharacter.FirstPersonCharacter_C|GethaveNarratorSound? (Variables|Default|GetrefChara))
        (Audio|Components|Audio|SetVolumeMultiplier _sound 0.01 :!class /Script/Engine.AudioComponent)
        (else
          (Audio|Components|Audio|SetVolumeMultiplier _sound 1.0 :!class /Script/Engine.AudioComponent))))))

(fn ConstructionScript)