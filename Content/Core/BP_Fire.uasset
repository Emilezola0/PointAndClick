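; BP_Fire is a fire actor that plays a spatialized fire sound at its own location.
; On BeginPlay it caches the first-person character, waits briefly, then uses the Otherdimension flag to pick the normal or other-dimension cue.
; The spawned audio component is stored with auto-destroy off and uses the SA_radio attenuation settings.
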(event EventBeginPlay
  (bind _returnvalue (Transformation|GetActorLocation))
  (bind _asfirst_person_character (Utilities|Casting|CastToFirstPersonCharacter (Game|GetPlayerCharacter 0))
    (:then
      (Variables|Default|SetrefChara _asfirst_person_character))
    (:CastFailed
      _))
  (Utilities|FlowControl|Delay 5.0)
  (if (Variables|Default|GetOtherdimension)
    (bind _returnvalue_2 (Audio|SpawnSoundatLocation "/Game/Sound/Fire_Cue_OtherDim.Fire_Cue_OtherDim" _returnvalue "0, 0, 0" 1.0 1.0 0.0 "/Game/Core/SA_radio.SA_radio" 0 false))
    (bind _output_get (Variables|Default|SetSound _returnvalue_2))
    (Audio|Components|Audio|Play _output_get 0.0)
    (else
      (bind _returnvalue_3 (Audio|SpawnSoundatLocation "/Game/Sound/Fire_Cue.Fire_Cue" _returnvalue "0, 0, 0" 1.0 1.0 0.0 "/Game/Core/SA_radio.SA_radio" 0 false))
      (bind _output_get_2 (Variables|Default|SetSound _returnvalue_3))
      (Audio|Components|Audio|Play _output_get_2 0.0))))

(fn ConstructionScript)