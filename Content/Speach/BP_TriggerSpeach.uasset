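; BP_TriggerSpeach is a trigger box that plays a one-time narrator line hinting that the player cannot force a door and should look for clues elsewhere.
; When the FirstPersonCharacter first overlaps the box, a Dialogue call shows typed text with 3D sound at the character's location.
; It removes the returned widget after the delay that call supplies.
; An older PlaySoundAtLocation and Delay chain remains unconnected.
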(event OnComponentBeginOverlap(Box)
  (params (OverlappedComponent :type Primitive%20Component%20Object%20Reference) (OtherActor :type Actor%20Object%20Reference) (OtherComp :type Primitive%20Component%20Object%20Reference) (OtherBodyIndex :type Integer) (bFromSweep :type Boolean) (SweepResult :type Hit%20Result%20Structure%20%28by%20ref%29))
  (bind _asfirst_person_character (Utilities|Casting|CastToFirstPersonCharacter OtherActor))
  (Utilities|FlowControl|DoOnce false
    (:Completed
      (bind (_delay_before_remove_widget _widget_reference) (CallFunction|Dialogue "Narrator" "Oh, look at you, you clever player! Trying to force your way through that door with your infallible ingenuity? Alas, you'll only bruise your pride. You'll need more than brawn to get out of here, so look elsewhere for clues." 0.08 true (Variables|Default|GetSpeach) 1.0 1.0 (Transformation|GetActorLocation _asfirst_person_character) false 0.0))
      (bind _output_get (Variables|Default|SetWidget%20Reference _widget_reference))
      (Utilities|FlowControl|Delay _delay_before_remove_widget)
      (Widget|RemovefromParent _output_get))))

(fn ConstructionScript)