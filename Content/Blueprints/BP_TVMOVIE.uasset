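; BP_TVMOVIE is a TV movie player that cycles endlessly through a list of media sources once its PLAY event fires.
; PLAY binds the media sound component to MP_AKIRA, waits an initial delay, then opens each source and holds it for its matching TIMER entry plus padding.
; Despite its name, the Random index advances sequentially and wraps to zero.
; BeginPlay clears the sound's player; its OtherDim branch does nothing.
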(event Custom|PLAY
  (Media|MediaSoundComponent|SetMediaPlayer (Variables|Default|GetMediaSound) "/Game/Movies/MP_AKIRA.MP_AKIRA")
  (Utilities|FlowControl|Delay 16.0)
  (if (<= (+ (Variables|Default|Getrandom) 1) (- (Utilities|Array|Length (Variables|Default|GetMedia%20Source)) 1)) :!label _label
    (Variables|Default|Setrandom (+ (Variables|Default|Getrandom) 1))
    (else
      (Variables|Default|Setrandom 0)))
  (Media|MediaPlayer|OpenSource (Variables|Default|Getmediaplayer) (Utilities|Array|Get(acopy) (Variables|Default|GetMedia%20Source) (Variables|Default|Getrandom)))
  (Utilities|FlowControl|Delay (+ (Utilities|Array|Get(acopy) (Variables|Default|GetTIMER) (Variables|Default|Getrandom)) 0.5))
  (Variables|Default|Setnoperandom (Variables|Default|Getrandom))
  (goto _label))

(event EventBeginPlay
  (if (Variables|Default|GetOtherDim?)
    _
    (else
      _))
  (Media|MediaSoundComponent|SetMediaPlayer (Variables|Default|GetMediaSound) 0))

(fn ConstructionScript)