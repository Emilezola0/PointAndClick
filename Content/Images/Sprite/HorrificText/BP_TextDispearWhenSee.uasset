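; BP_TextDispearWhenSee is an actor, named as horrific text that disappears when seen, whose visibility follows the player's facing direction.
; BeginPlay caches the player's FirstPersonCharacter.
; Every Tick, it hides itself while that character's world yaw is beyond 80 degrees either side of zero and shows itself otherwise.
; The check uses absolute rotation only, ignoring the actor's position and line of sight.
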(event EventTick
  (params (DeltaSeconds :type Float%20%28single-precision%29))
  (bind _as_first_person_character (Variables|Default|GetAs%20First%20Person%20Character))
  (bind _returnvalue (Transformation|GetActorRotation _as_first_person_character))
  (bind _yaw (Math|Rotator|BreakRotator _returnvalue))
  (if (or (> _yaw 8e+01) (< _yaw -8e+01))
    (Rendering|SetActorHiddenInGame true)
    (else
      (Rendering|SetActorHiddenInGame false))))

(event EventBeginPlay
  (bind _asfirst_person_character (Utilities|Casting|CastToFirstPersonCharacter (Game|GetPlayerCharacter 0)))
  (Variables|Default|SetAs%20First%20Person%20Character _asfirst_person_character))

(fn ConstructionScript)